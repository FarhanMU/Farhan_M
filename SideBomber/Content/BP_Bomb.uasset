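; BP_Bomb is a timed bomb actor that grows, then explodes in four directions.
; On BeginPlay the ScaleUp timeline drives the sphere's uniform scale and calls Explode when it finishes.
; Explode spawns a BP_Explosion at the sphere's location facing each positive and negative X and Y world axis, then destroys the bomb.
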(event `self.ReceiveBeginPlay`
  (bind (_direction _alpha) (`Timeline|ScaleUp`)
    (:`Update`
      (`SceneComponent.SetRelativeScale3D` (`self.Sphere`) (`KismetMathLibrary.Conv_DoubleToVector` _alpha)))
    (:`Finished`
      (`self.explode`))))

(event `explode`
  (for _array_element (`|MakeArray` (1.0 0.0 0.0) (0.0 1.0 0.0) (-1.0 0.0 0.0) (0.0 -1.0 0.0) :!type "Vector Structure")
    (`|SpawnActorFromClass` "/Game/BP_Explosion.BP_Explosion_C" (`KismetMathLibrary.MakeTransform` (`SceneComponent.K2_GetComponentLocation` (`self.Sphere`)) (`KismetMathLibrary.Conv_VectorToRotator` _array_element)) "Undefined" "OverrideRootScale" null null))
  (`self.K2_DestroyActor`))

(fn `UserConstructionScript`)