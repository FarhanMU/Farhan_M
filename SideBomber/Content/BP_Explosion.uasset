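; BP_Explosion is a traveling explosion that destroys side-scroller characters, walls and three enemy types it overlaps.
; On BeginPlay a forward box trace against WorldStatic objects shortens its travel Length to the first hit.
; Tick sweeps it forward at Speed until it has covered that Length, then stops and destroys it.
; While moving, Box overlaps cast the other actor to each supported class and destroy it.
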(event `self.ReceiveBeginPlay`
  (bind _startlocation (`self.StartLocation`))
  (set `self.StartLocation` (`self.K2_GetActorLocation`))
  (bind (_outhit _returnvalue) (`KismetSystemLibrary.BoxTraceSingleForObjects` _startlocation (+ _startlocation (* (`self.GetActorForwardVector`) (`self.length`))) (20.0 20.0 20.0) (struct) (`|MakeArray` "ObjectTypeQuery1" :!type "EObjectTypeQuery Enum")))
  (if _returnvalue
    (set `self.length` (`.Distance` (`GameplayStatics.BreakHitResult` _outhit)))))

(event `self.ReceiveTick`
  (params (DeltaSeconds :type "Float (single-precision)"))
  (if (not (`self.stop?`))
    (`self.K2_AddActorWorldOffset` (* (`self.GetActorForwardVector`) (* DeltaSeconds (`self.speed`))) true)
    (if (>= (`KismetMathLibrary.VSize` (- (`self.StartLocation`) (`self.K2_GetActorLocation`))) (`self.length`))
      (set `self.stop?` true)
      (`KismetSystemLibrary.Delay` 0.0001)
      (`self.K2_DestroyActor`))))

(event `self.Box.OnComponentBeginOverlap`
  (params (OverlappedComponent :type "PrimitiveComponent Object Reference") (OtherActor :type "Actor Object Reference") (OtherComp :type "PrimitiveComponent Object Reference") (OtherBodyIndex :type Integer) (bFromSweep :type Boolean) (SweepResult :type "HitResult Structure (by ref)"))
  (if (not (`self.stop?`))
    (`|ExecutionSequence`
      (:`then_0`
        (bind _asside_scroller_character (cast `/Game/SideScrollerBP/Blueprints/SideScrollerCharacter` OtherActor))
        (`self.K2_DestroyActor` _asside_scroller_character))
      (:`then_1`
        (bind _aswall (cast `/Game/Wall` OtherActor))
        (`self.K2_DestroyActor` _aswall))
      (:`then_2`
        (bind _asenemy (cast `/Game/Enemy` OtherActor))
        (`self.K2_DestroyActor` _asenemy))
      (:`then_3`
        (bind _asenemy_2 (cast `/Game/enemy2` OtherActor))
        (`self.K2_DestroyActor` _asenemy_2))
      (:`then_4`
        (bind _asenemy_3 (cast `/Game/enemy3` OtherActor))
        (`self.K2_DestroyActor` _asenemy_3)))))

(fn `UserConstructionScript`)